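; Base AI controller for KGCharacterBase pawns that seeks health, hunts players and wanders, using Blueprint logic instead of a behavior tree.
; A looping timer runs ProcessAI, which first sends a pawn below its class-default health toward a nearby health pickup.
; Otherwise it keeps or finds a player Target by sphere overlap, moves into AttackRange and uses its primary attack.
; With no target, it wanders to random navigable points.
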(event Custom|Wonder
  (bind _returnvalue (Pawn|GetControlledPawn))
  (Utilities|IsValid _returnvalue
    (:Is%20Valid
      (AI|AIMoveTo _returnvalue (.RandomLocation (Class|NavigationSystemV1|GetRandomPointinNavigableRadius (Transformation|GetActorLocation _returnvalue) 2e+03 0 0)) 0 5.0 false))))

(event Custom|ProcessAI
  (bind _returnvalue (Pawn|GetControlledPawn))
  (bind _askgcharacter_base (Utilities|Casting|CastToKGCharacterBase (Pawn|GetControlledPawn))
    (:then
      (if (< (Variables|/Game/Blueprints/KGCharacterBase.KGCharacterBase_C|GetHealth _askgcharacter_base) (.Health (Utilities|GetClassDefaults (Utilities|GetClass _askgcharacter_base))))
        (bind (_outactors _returnvalue_2) (Collision|SphereOverlapActors (Transformation|GetActorLocation (Pawn|GetControlledPawn)) 1e+03 (Utilities|Array|MakeArray "ObjectTypeQuery2") "/Game/Blueprints/KGHealthPickup.KGHealthPickup_C"))
        (if _returnvalue_2
          (AI|AIMoveTo _returnvalue "0, 0, 0" (Utilities|Array|Get(acopy) _outactors) 2e+01 false)
          (else
            (Variables|Default|GetTarget :!label _label
              (:then
                (AI|AIMoveTo _returnvalue "0, 0, 0" (Variables|Default|GetTarget) (Variables|/Game/Blueprints/KGCharacterBase.KGCharacterBase_C|GetAttackRange (.AsKGCharacter%20Base (Utilities|Casting|CastToKGCharacterBase _returnvalue))) false :!label _label_2
                  (:OnSuccess
                    (bind _askgcharacter_base_2 (Utilities|Casting|CastToKGCharacterBase (Pawn|GetControlledPawn)))
                    (AI|SetFocalPoint (Transformation|GetActorLocation (Variables|Default|GetTarget)))
                    (Default|UsePrimaryAttack _askgcharacter_base_2))))
              (:else
                (bind _outactors_2 (Collision|SphereOverlapActors (Transformation|GetActorLocation) 1e+03 (Utilities|Array|MakeArray "ObjectTypeQuery3") 0 (Utilities|Array|MakeArray (Pawn|GetControlledPawn))))
                (bind _array_element (Utilities|Array|ForEachLoopwithBreak _outactors_2 :!label _label_3)
                  (:LoopBody
                    (bind _askgcharacter_base_3 (Utilities|Casting|CastToKGCharacterBase _array_element))
                    (if (Class|Controller|IsPlayerController (Pawn|GetController _askgcharacter_base_3))
                      (Variables|Default|SetTarget _askgcharacter_base_3)
                      (goto _label_3 Break)))
                  (:Completed
                    (Variables|Default|GetTarget
                      (:then
                        (goto _label_2))
                      (:else
                        (CallFunction|Wonder)))))))))
        (else
          (goto _label))))
    (:CastFailed
      (goto _label))))

(event EventBeginPlay
  (Utilities|Time|SetTimerbyEvent (delegate Custom|ProcessAI) 2.0 true))

(event EventTick
  (params (DeltaSeconds :type Float%20%28single-precision%29)))

(fn ConstructionScript)